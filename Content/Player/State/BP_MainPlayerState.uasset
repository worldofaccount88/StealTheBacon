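; Player state Blueprint that relays game phase changes (Lobby, StartGame, InProgress, EndPhase) to the player's HUD.
; Each phase has an Init event that forwards to a Run on Client RPC, which calls the matching phase message function on the local HUD.
; GetGamePhase returns a fixed enum value rather than a tracked phase, and the phase-change warning prints are disconnected.
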(event Custom|RunOnClient%20:%20Init%20EndPhase
  ;[1 1 1] Init EndPhase
  (Class|BPILobbyHandling|InitEndPhase(Message) (HUD|GetHUD (Game|GetPlayerController))))

(event Custom|RunOnClient%20:%20Init%20LobbyPhase
  ;[1 1 1] Init Lobby Phase
  (Class|BPILobbyHandling|InitLobbyPhase(Message) (HUD|GetHUD (Game|GetPlayerController))))

(event Custom|RunOnClient%20:%20Init%20StartPhase
  ;[1 1 1] Init StartGame Phase
  (Class|BPILobbyHandling|InitStartGame(Message) (HUD|GetHUD (Game|GetPlayerController))))

(event Custom|RunOnClient%20:%20Init%20InProgress
  ;[1 1 1] Init InProgress Phase
  (Class|BPILobbyHandling|InitinProgress(Message) (HUD|GetHUD (Game|GetPlayerController))))

(event EventInitLobbyPhase
  ;[1 1 1] Init Lobby Phase
  (CallFunction|RunonClient:InitLobbyPhase))

(event EventInitStartGame
  ;[1 1 1] Init StartGame Phase
  (CallFunction|RunonClient:InitStartPhase))

(event EventInitinProgress
  ;[1 1 1] Init InProgress Phase
  (CallFunction|RunonClient:InitinProgress))

(event EventInitEndPhase
  ;[1 1 1] Init EndPhase
  (CallFunction|RunonClient:InitEndPhase))

(fn ConstructionScript)

(fn GetGamePhase
  (return "NewEnumerator0"))