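; Game mode that tracks the players who join the match.
; On PostLogin with authority, it pairs each valid PlayerState with its unique ID and appends the entry to PlayerControllerList.
; It then passes the whole list to the game state through UpdatePlayerListMessage.
; GetPlayerList is an empty stub.
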(event EventPostLogin
  (params (NewPlayer :type Player%20Controller%20Object%20Reference))
  ;[1 1 1] Update Player List on Server Game State
  (Networking|SwitchHasAuthority
    (:Authority
      (bind _playerstate (Variables|/Script/Engine.Controller|GetPlayerState NewPlayer)
        (:then
          (bind _output_get (Variables|Default|SetNewPlayerStruct (Utilities|Struct|MakeS_PlayerInfo _playerstate (PlayerState|GetUniqueID _playerstate))))
          (Utilities|Array|Add (Variables|Default|GetPlayerControllerList) _output_get)
          (Networking|SwitchHasAuthority
            (:Authority
              (Class|BPIPlayerHandling|UpdatePlayerList(Message) (Game|GetGameState) (Variables|Default|GetPlayerControllerList)))))
        (:else)))))

(fn ConstructionScript)

(fn GetPlayerList
  (return 0))