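; Main game state Blueprint that tracks the match phase: lobby, start game, in progress or end.
; ChangeGamePhaseto passes the phase to SetOnClients, stores it, then runs the matching Init event, which sends that phase's message to every entry in PlayerArray.
; UpdatePlayerList replaces the stored player info map, and GetGamePhase exposes the current phase.
; OnRep_GamePhase is empty, and the warning prints are never run.
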(event Custom|SetOnClients
  (params (GamePhase :type E_GamePhase%20Enum :default "NewEnumerator0"))
  (Variables|Default|SetGamePhase GamePhase))

(event EventChangeGamePhaseto
  (params (DesiredPhase :type E_GamePhase%20Enum :default "NewEnumerator0"))
  (CallFunction|SetonClients DesiredPhase)
  (bind _output_get (Variables|Default|SetGamePhase DesiredPhase))
  (switch Utilities|FlowControl|Switch|SwitchonE_GamePhase _output_get
    (:NewEnumerator0
      ;[1 1 1] Phase Change  calls to delegates
      (CallFunction|InitLobbyPhase))
    (:NewEnumerator1
      (CallFunction|InitStartGame))
    (:NewEnumerator2
      (CallFunction|InitinProgress))
    (:NewEnumerator3
      (CallFunction|InitEndPhase))))

(event EventInitLobbyPhase
  ;[1 1 1] Phase change delegates
  ;[1 1 1] Comment
  (for _array_element (Variables|Default|GetPlayerArray)
    (Class|BPILobbyHandling|InitLobbyPhase(Message) _array_element)))

(event EventInitinProgress
  ;[1 1 1] Phase change delegates
  ;[1 1 1] Init InProgress
  (for _array_element (Variables|Default|GetPlayerArray)
    (Class|BPILobbyHandling|InitinProgress(Message) _array_element)))

(event EventInitStartGame
  ;[1 1 1] Phase change delegates
  ;[1 1 1] Init StartGame
  (for _array_element (Variables|Default|GetPlayerArray)
    (Class|BPILobbyHandling|InitStartGame(Message) _array_element)))

(event EventInitEndPhase
  ;[1 1 1] Phase change delegates
  ;[1 1 1] Init EndPhase
  (for _array_element (Variables|Default|GetPlayerArray)
    (Class|BPILobbyHandling|InitEndPhase(Message) _array_element)))

(event EventUpdatePlayerList
  (params (PlayerInfoMap :type Map%20of%20Strings%20to%20Structs))
  (Variables|Default|SetPlayer%20Info%20Map PlayerInfoMap))

(fn ConstructionScript)

(fn OnRepGamePhase)

(fn GetGamePhase
  (return (Variables|Default|GetGamePhase)))