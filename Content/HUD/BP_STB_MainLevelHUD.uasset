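; BP_STB_MainLevelHUD is the main level HUD that shows a different widget for each game phase.
; BeginPlay and the lobby, start, in-progress and end phase events all call ChangeHUD and store the resulting widget.
; ChangeHUD reads the phase from the GameState, removes the current widget, then creates one from a class array indexed by that phase.
; UpdatePlayerList forwards a refresh message to the active widget.
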(event EventBeginPlay
  ;[1 1 1] Starts in Lobby view
  (bind _newuserwidget (CallFunction|ChangeHUD))
  (Variables|Default|SetUserWidget _newuserwidget))

(event EventInitLobbyPhase
  (bind _newuserwidget (CallFunction|ChangeHUD))
  (Variables|Default|SetUserWidget _newuserwidget))

(event EventUpdatePlayerList
  (params (PlayerInfoArray :type Array%20of%20S%20Player%20Info%20Structures))
  (Class|BPIPlayerHandling|UpdatePlayerList(Message) (Variables|Default|GetUserWidget)))

(event EventInitStartGame
  (bind _newuserwidget (CallFunction|ChangeHUD))
  (Variables|Default|SetUserWidget _newuserwidget))

(event EventInitinProgress
  (bind _newuserwidget (CallFunction|ChangeHUD))
  (Variables|Default|SetUserWidget _newuserwidget))

(event EventInitEndPhase
  (bind _newuserwidget (CallFunction|ChangeHUD))
  (Variables|Default|SetUserWidget _newuserwidget))

(fn ConstructionScript)

(fn ChangeHUD
  (bind _gamephase (Class|BPILobbyHandling|GetGamePhase(Message) (Game|GetGameState)))
  (LocalVariables|SetGamePhaseVar _gamephase)
  (bind _userwidget (Variables|Default|GetUserWidget)
    (:then
      (Widget|RemovefromParent _userwidget))
    (:else
      _))
  (bind _returnvalue (UserInterface|CreateWidget (Utilities|Array|Get(acopy) (Variables|Default|GetWidgetClassChoice) (Math|Conversions|ToInteger(Byte) (LocalVariables|GetGamePhaseVar)))))
  (Utilities|IsValid _returnvalue
    (:Is%20Valid
      (UserInterface|Viewport|AddtoViewport _returnvalue 0)
      (return _returnvalue))
    (:Is%20Not%20Valid
      (return 0))))

(fn GetGamePhase
  (return "NewEnumerator0"))

(fn GetPlayerInfo
  (return ""))

(fn GetPlayersTeams
  (return 0))